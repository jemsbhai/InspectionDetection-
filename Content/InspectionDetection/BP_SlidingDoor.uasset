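; BP_SlidingDoor is a door that slides along its local X axis when inspected.
; OnInspect plays or reverses a timeline based on DoorOpen, and the track value sets the mesh's relative location.
; DoorOpen comes from a FlipFlop on the timeline's Update, so it toggles every update rather than once per inspection.
; A second timeline that offsets from the current X is left unconnected.
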(event EventOnInspect
  (if (Variables|Default|GetDoorOpen)
    (bind _newtrack_0 (Timeline|Timeline Reverse)
      (:Update
        (Transformation|SetRelativeLocation (Variables|Default|GetDoorMesh) (Math|Vector|MakeVector _newtrack_0 0.0 0.0) false false)
        (bind _isa (Utilities|FlowControl|FlipFlop)
          (:A
            _)
          (:B
            _))
        (Variables|Default|SetDoorOpen _isa)))
    (else
      (Timeline|Timeline Play))))

(fn ConstructionScript)