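; BP_Inspectable is an inspectable world actor that brings up a shared interaction menu when inspected.
; OnInspect fetches the InteractMenu actor from IDGameInstance, unhides it and moves it to this actor's root.
; It turns the menu toward the player using the camera forward vector with X and Y negated, nudges it along that facing, then passes itself to the menu's select event.
; The player raycast hit event is an empty stub.
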(event EventBeginPlay)

(event Collision|EventActorBeginOverlap
  (params (OtherActor :type Actor%20Object%20Reference)))

(event EventTick
  (params (DeltaSeconds :type Float%20%28single-precision%29)))

(event EventOnRaycastHitbyPlayer)

(event EventOnInspect
  (bind _asidgame_instance (Utilities|Casting|CastToIDGameInstance (Game|GetGameInstance)))
  (Rendering|SetActorHiddenInGame (Variables|/Game/InspectionDetection/IDGameInstance.IDGameInstance_C|GetInteractMenu _asidgame_instance) false)
  (Transformation|SetActorLocation (Variables|/Game/InspectionDetection/IDGameInstance.IDGameInstance_C|GetInteractMenu _asidgame_instance) (Transformation|GetWorldLocation (Variables|Default|GetDefaultSceneRoot)) false false)
  (bind _asbp_first_person_character (Utilities|Casting|CastToBP_FirstPersonCharacter (Pawn|GetControlledPawn (Game|GetPlayerController 0))))
  (Transformation|SetActorRotation (Variables|/Game/InspectionDetection/IDGameInstance.IDGameInstance_C|GetInteractMenu _asidgame_instance) (Math|Conversions|RotationFromXVector (* (Math|Vector|GetForwardVector (Variables|/Game/InspectionDetection/BP_FirstPersonCharacter.BP_FirstPersonCharacter_C|GetFirstPersonCamera _asbp_first_person_character)) "-1.000000,-1.000000,1.000000")))
  (Transformation|SetActorLocation (Variables|/Game/InspectionDetection/IDGameInstance.IDGameInstance_C|GetInteractMenu _asidgame_instance) (+ (Transformation|GetWorldLocation (Variables|/Script/Engine.Actor|GetRootComponent (Variables|/Game/InspectionDetection/IDGameInstance.IDGameInstance_C|GetInteractMenu _asidgame_instance))) (* (Math|Vector|GetForwardVector (Transformation|GetWorldRotation (Variables|/Script/Engine.Actor|GetRootComponent (Variables|/Game/InspectionDetection/IDGameInstance.IDGameInstance_C|GetInteractMenu _asidgame_instance)))) 7e+01)) false false)
  (Default|OnSelectEventEvent (Variables|/Game/InspectionDetection/IDGameInstance.IDGameInstance_C|GetInteractMenu _asidgame_instance) self))

(fn ConstructionScript)